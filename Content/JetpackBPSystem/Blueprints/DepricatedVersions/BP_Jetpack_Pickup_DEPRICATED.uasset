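; Deprecated jetpack pickup actor that equips a jetpack on the player who overlaps it.
; On overlap it casts the other actor to the deprecated first-person character, then the third-person one, and on a match destroys itself and calls that character's EquipJetpack.
; If neither cast succeeds, an optional debug flag prints a warning with the pickup's own display name.
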(event `self.ReceiveActorBeginOverlap`
  (params (OtherActor :type "Actor Object Reference"))
  (bind _asbp_jetpack_first_person_character_depricated (cast `/Game/JetpackBPSystem/Blueprints/DepricatedVersions/BP_Jetpack_FirstPersonCharacter_DEPRICATED` OtherActor) ; Check to see if wer're specifically interacting with the first person character.
    (:`then`
      (`self.K2_DestroyActor`) ; Destroy power up.
      (`/Game/JetpackBPSystem/Blueprints/DepricatedVersions/BP_Jetpack_FirstPersonCharacter_DEPRICATED.Equip Jetpack` _asbp_jetpack_first_person_character_depricated) ; Perform the Equip Jetpack function on the player. This will active the jetpack component on them, rather than
    )
    (:`CastFailed`
      (bind _asbp_jetpack_third_person_character_depricated (cast `/Game/JetpackBPSystem/Blueprints/DepricatedVersions/BP_Jetpack_ThirdPersonCharacter_DEPRICATED` OtherActor) ; Or the Third Person Character.
        (:`then`
          (`self.K2_DestroyActor`)
          (`/Game/JetpackBPSystem/Blueprints/DepricatedVersions/BP_Jetpack_ThirdPersonCharacter_DEPRICATED.Equip Jetpack` _asbp_jetpack_third_person_character_depricated))
        (:`CastFailed`
          ;[1 1 1] Debug
          (if (`self.Debug: Can't Find Player`)
            (`KismetSystemLibrary.PrintString` (`KismetStringLibrary.Concat_StrStr` (`KismetSystemLibrary.GetDisplayName` self) ": Is not casting to player. Check if casts are for correct objects?"))))))))

(fn `UserConstructionScript`)