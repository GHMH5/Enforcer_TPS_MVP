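; Actor component that gives a pawn a configurable jetpack or multi-jump, with optional editor example presets applied at BeginPlay.
; Jump or Jetpack input messages, chosen by input method, start thrust via negative gravity or repeated impulses, or launch capped air jumps.
; Delay loops drain fuel in flight and refill it on the ground.
; A ticked landing check resets jump count, gravity and air control, avoiding reliance on animation events.
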(event `self.ReceiveBeginPlay`
  (bind _character_movement (`self.Character Movement`))
  ;[1 0 0] Establish Character Movement Controller
  (bind _aspawn (cast `Pawn` (`self.GetOwner`)))
  (set `self.Character Movement` (`Actor.GetComponentByClass` _aspawn "/Script/Engine.CharacterMovementComponent"))
  ;[1 0 0] Jetpack Setup
  (set `self.Base Gravity` (`CharacterMovementComponent.GravityScale` _character_movement)) ; Set base gravity.
  (set `self.Base Air Control` (`CharacterMovementComponent.AirControl` _character_movement)) ; Set base air control.
  (if (> (`self.Starting Fuel`) (`self.Max Fuel`))
    (set `self.Starting Fuel` (`self.Max Fuel`)))
  (set `self.Current Fuel` (`self.Starting Fuel`)) ; Make sure the current and starting fuel are the same.
  ;[1 0 0] Example presets
  (switch `/Game/JetpackBPSystem/Blueprints/Enum_JetpackExamples` (`self.Example Preset`) ; The example presets enum is used in the editor to set the following variable strings up.\nIt is not intended for use in full development, and this section can be deleted without repercussion.
    (:`NewEnumerator0`
      _)
    (:`NewEnumerator1`
      ;[1 1 1] Example Presets
      ;;[1 0 0] Equip Jetpack
      (set `self.Jetpack Equipped` true)
      ;;[1 0 0] Input Method
      (set `self.Input Method` "NewEnumerator0")
      ;;[1 0 0] Flight Control
      (set `self.Flight Thrust` 2.0)
      (set `self.Flight Air Control` 1.0)
      ;;[1 0 0] Fall Gravity
      (set `self.Fall Gravity` 0.0)
      ;;[1 0 0] Fuel Settings
      (set `self.Max Fuel` 500.0)
      (set `self.Starting Fuel` 500.0)
      (set `self.Current Fuel` 500.0)
      (set `self.Fuel Consumption Amount` 10.0)
      (set `self.Fuel Consumption Rate` 0.1)
      ;;[1 0 0] Refuel settings
      (set `self.Refuel on Ground` true)
      (set `self.Ground Refuel Amount` 1.0)
      (set `self.Ground Refuel Rate` 1.0)
      ;;[1 0 0] Double Jump
      (set `self.Max Number of Jumps` 0)
      (set `self.Double Jump Strength` 0.0)
      (set `self.Double Jump End Delay` 0.0)
      (set `self.Air Control Reset` true)
      ;;[1 0 0] Debug
      (set `self.Debug: Print Out Fuel Levels` true)
      (`self.CEv: Refuel Check`))
    (:`NewEnumerator2`
      ;;[1 0 0] Equip Jetpack
      (set `self.Jetpack Equipped` true)
      ;;[1 0 0] Input Method
      (set `self.Input Method` "NewEnumerator0")
      ;;[1 0 0] Flight Control
      (set `self.Flight Thrust` 20.0)
      (set `self.Flight Air Control` 1.0)
      ;;[1 0 0] Fall Gravity
      (set `self.Fall Gravity` 1.25)
      ;;[1 0 0] Fuel Settings
      (set `self.Max Fuel` 500.0)
      (set `self.Starting Fuel` 500.0)
      (set `self.Current Fuel` 500.0)
      (set `self.Fuel Consumption Amount` 500.0)
      (set `self.Fuel Consumption Rate` 0.1)
      ;;[1 0 0] Refuel settings
      (set `self.Refuel on Ground` true)
      (set `self.Ground Refuel Amount` 2.0)
      (set `self.Ground Refuel Rate` 0.01)
      ;;[1 0 0] Double Jump
      (set `self.Max Number of Jumps` 0)
      (set `self.Double Jump Strength` 0.0)
      (set `self.Double Jump End Delay` 0.0)
      (set `self.Air Control Reset` true)
      ;;[1 0 0] Debug
      (set `self.Debug: Print Out Fuel Levels` true)
      (`self.CEv: Refuel Check`))
    (:`NewEnumerator3`
      ;;[1 0 0] Equip Jetpack
      (set `self.Jetpack Equipped` true)
      ;;[1 0 0] Input Method
      (set `self.Input Method` "NewEnumerator0")
      ;;[1 0 0] Flight Control
      (set `self.Flight Thrust` 0.0)
      (set `self.Flight Air Control` 1.0)
      ;;[1 0 0] Fall Gravity
      (set `self.Fall Gravity` 0.0)
      ;;[1 0 0] Fuel Settings
      (set `self.Max Fuel` 200.0)
      (set `self.Starting Fuel` 100.0)
      (set `self.Current Fuel` 100.0)
      (set `self.Fuel Consumption Amount` 1.0)
      (set `self.Fuel Consumption Rate` 0.1)
      ;;[1 0 0] Refuel settings
      (set `self.Refuel on Ground` true)
      (set `self.Ground Refuel Amount` 1.0)
      (set `self.Ground Refuel Rate` 0.05)
      ;;[1 0 0] Double Jump
      (set `self.Max Number of Jumps` 0)
      (set `self.Double Jump Strength` 0.0)
      (set `self.Double Jump End Delay` 0.0)
      (set `self.Air Control Reset` true)
      ;;[1 0 0] Debug
      (set `self.Debug: Print Out Fuel Levels` true)
      (`self.CEv: Refuel Check`))
    (:`NewEnumerator5`
      ;;[1 0 0] Equip Jetpack
      (set `self.Jetpack Equipped` true)
      ;;[1 0 0] Input Method
      (set `self.Input Method` "NewEnumerator0")
      ;;[1 0 0] Flight Control
      (set `self.Flight Thrust` -0.2)
      (set `self.Flight Air Control` 1.0)
      ;;[1 0 0] Fall Gravity
      (set `self.Fall Gravity` 0.0)
      ;;[1 0 0] Fuel Settings
      (set `self.Max Fuel` 500.0)
      (set `self.Starting Fuel` 500.0)
      (set `self.Current Fuel` 500.0)
      (set `self.Fuel Consumption Amount` 25.0)
      (set `self.Fuel Consumption Rate` 0.1)
      ;;[1 0 0] Refuel settings
      (set `self.Refuel on Ground` true)
      (set `self.Ground Refuel Amount` 500.0)
      (set `self.Ground Refuel Rate` 0.25)
      ;;[1 0 0] Double Jump
      (set `self.Max Number of Jumps` 0)
      (set `self.Double Jump Strength` 0.0)
      (set `self.Double Jump End Delay` 0.0)
      (set `self.Air Control Reset` true)
      ;;[1 0 0] Debug
      (set `self.Debug: Print Out Fuel Levels` true)
      (`self.CEv: Refuel Check`))
    (:`NewEnumerator4`
      ;;[1 0 0] Equip Jetpack
      (set `self.Jetpack Equipped` true)
      ;;[1 0 0] Input Method
      (set `self.Input Method` "NewEnumerator0")
      ;;[1 0 0] Flight Control
      (set `self.Flight Thrust` 0.2)
      (set `self.Flight Air Control` 1.0)
      ;;[1 0 0] Fall Gravity
      (set `self.Fall Gravity` 2.5)
      ;;[1 0 0] Fuel Settings
      (set `self.Max Fuel` 1500.0)
      (set `self.Starting Fuel` 1500.0)
      (set `self.Current Fuel` 1500.0)
      (set `self.Fuel Consumption Amount` 20.0)
      (set `self.Fuel Consumption Rate` 0.1)
      ;;[1 0 0] Refuel settings
      (set `self.Refuel on Ground` false)
      (set `self.Ground Refuel Amount` 2.0)
      (set `self.Ground Refuel Rate` 0.01)
      ;;[1 0 0] Double Jump
      (set `self.Max Number of Jumps` 0)
      (set `self.Double Jump Strength` 0.0)
      (set `self.Double Jump End Delay` 0.0)
      (set `self.Air Control Reset` true)
      ;;[1 0 0] Debug
      (set `self.Debug: Print Out Fuel Levels` true)
      (`self.CEv: Refuel Check`))
    (:`NewEnumerator6`
      ;;[1 0 0] Equip Jetpack
      (set `self.Jetpack Equipped` true)
      ;;[1 0 0] Input Method
      (set `self.Input Method` "NewEnumerator0")
      ;;[1 0 0] Flight Control
      (set `self.Flight Thrust` 0.0)
      (set `self.Flight Air Control` 1.0)
      ;;[1 0 0] Fall Gravity
      (set `self.Fall Gravity` 0.25)
      ;;[1 0 0] Fuel Settings
      (set `self.Max Fuel` 0.0)
      (set `self.Starting Fuel` 0.0)
      (set `self.Current Fuel` 0.0)
      (set `self.Fuel Consumption Amount` 0.0)
      (set `self.Fuel Consumption Rate` 0.0)
      ;;[1 0 0] Refuel settings
      (set `self.Refuel on Ground` false)
      (set `self.Ground Refuel Amount` 0.0)
      (set `self.Ground Refuel Rate` 0.0)
      ;;[1 0 0] Double Jump
      (set `self.Max Number of Jumps` 2)
      (set `self.Double Jump Strength` 1200.0)
      (set `self.Double Jump End Delay` 0.1)
      (set `self.Air Control Reset` true)
      ;;[1 0 0] Debug
      (set `self.Debug: Print Out Fuel Levels` false)
      (`self.CEv: Refuel Check`))
    (:`NewEnumerator7`
      ;;[1 0 0] Equip Jetpack
      (set `self.Jetpack Equipped` true)
      ;;[1 0 0] Input Method
      (set `self.Input Method` "NewEnumerator0")
      ;;[1 0 0] Flight Control
      (set `self.Flight Thrust` 0.0)
      (set `self.Flight Air Control` 0.0)
      ;;[1 0 0] Fall Gravity
      (set `self.Fall Gravity` 1.0)
      ;;[1 0 0] Fuel Settings
      (set `self.Max Fuel` 0.0)
      (set `self.Starting Fuel` 0.0)
      (set `self.Current Fuel` 0.0)
      (set `self.Fuel Consumption Amount` 0.0)
      (set `self.Fuel Consumption Rate` 0.0)
      ;;[1 0 0] Refuel settings
      (set `self.Refuel on Ground` false)
      (set `self.Ground Refuel Amount` 0.0)
      (set `self.Ground Refuel Rate` 0.0)
      ;;[1 0 0] Double Jump
      (set `self.Max Number of Jumps` 3)
      (set `self.Double Jump Strength` 1000.0)
      (set `self.Double Jump End Delay` 0.5)
      (set `self.Air Control Reset` true)
      ;;[1 0 0] Debug
      (set `self.Debug: Print Out Fuel Levels` false)
      (`self.CEv: Refuel Check`))
    (:`NewEnumerator8`
      ;;[1 0 0] Equip Jetpack
      (set `self.Jetpack Equipped` true)
      ;;[1 0 0] Input Method
      (set `self.Input Method` "NewEnumerator0")
      ;;[1 0 0] Flight Control
      (set `self.Flight Thrust` 0.0)
      (set `self.Flight Air Control` 1.0)
      ;;[1 0 0] Fall Gravity
      (set `self.Fall Gravity` 5.0)
      ;;[1 0 0] Fuel Settings
      (set `self.Max Fuel` 0.0)
      (set `self.Starting Fuel` 0.0)
      (set `self.Current Fuel` 0.0)
      (set `self.Fuel Consumption Amount` 0.0)
      (set `self.Fuel Consumption Rate` 0.0)
      ;;[1 0 0] Refuel settings
      (set `self.Refuel on Ground` false)
      (set `self.Ground Refuel Amount` 0.0)
      (set `self.Ground Refuel Rate` 0.0)
      ;;[1 0 0] Double Jump
      (set `self.Max Number of Jumps` 9001)
      (set `self.Double Jump Strength` 300.0)
      (set `self.Double Jump End Delay` 1.0)
      (set `self.Air Control Reset` true)
      ;;[1 0 0] Debug
      (set `self.Debug: Print Out Fuel Levels` false)
      (`self.CEv: Refuel Check`)))
  ;[1 0 0] Jetpack check if we're refueling on the ground.
  (if (`self.Jetpack Equipped`)
    (if (`self.Refuel on Ground`)
      (`self.CEv: Refuel Check`) ; Start that processing.
    )))

(event `self.ReceiveTick`
  (params (DeltaSeconds :type "Float (single-precision)"))
  ;[1 0 0] Jetpack check if we're grounded or not.
  (`self.Jetpack Check Landed`) ; This function could be called from an Animation Blueprint,\nhowever, the landing animation is prone to being skiped\nwhen the player lands on a ledge. This is an acceptable\nalternative.
)

(event `/Game/JetpackBPSystem/Blueprints/BPI_Jetpack_ComponentCommunication.BPI Pressed Jump`
  (bind _current_fuel (`self.Current Fuel`))
  ;[1 0 0] Check if Jetpack is equipped.
  (if (`self.Jetpack Equipped`)
    ;[1 0 0] Check input method, from there, determine the course of action.
    (switch `/Game/JetpackBPSystem/Blueprints/Enum_JetpackInputMethod` (`self.Input Method`) ; Split the event processing based on what the Input Method is.
      (:`NewEnumerator0`
        ;[1 0 0] Timed lock so "Fall Gravity" doesn't kick in immediately after trying to jump.
        (if (`NavMovementComponent.IsFalling` (`self.Character Movement`))
          (set `self.Jump Count` (+ (`self.Jump Count`) 2.0)) ; Jumping in the air counts as "2".\nThis is set to 2, so that the player doesn't have to "jump" twice in the air\nif they want to use the jetpack after falling off a ledge and into open air.
          (else
            (set `self.Jump Count` (+ (`self.Jump Count`) 1.0)) ; Jumping from the ground counts as "1"
          ))
        (`KismetSystemLibrary.Delay` (`self.Jump Delay`)) ; Check if player is still trying to use the jetpack, after delay.\nWithout it, the player can activate the jetpack on the ground.
        (if (> (`self.Jump Count`) 1.0)
          ;[1 0 0] Do we use fuel?
          (if (> (`self.Max Fuel`) 0.0)
            ;[1 0 0] Set fuel usage.
            (set `self.Consuming Fuel` true :!label _label) ; This is the main variable used to determine\nwhen to shut off the fuel consuming cycle. It\nis turned on at the start here, and turned off\nbelow, where the player releases the input.
            ;[1 0 0] Check if we have enough fuel.
            (if (>= (`self.Current Fuel`) (`self.Fuel Consumption Amount`)) :!label _label_2
              ;[1 0 0] Activate / Deactivate Jetpack (fuel).
              (`self.Jetpack Thrust Begin`) ; This function carries out the actual boost.
              ;[1 0 0] Fuel consumption.
              (if (`self.Consuming Fuel`)
                (set `self.Current Fuel` (- (`self.Current Fuel`) (`self.Fuel Consumption Amount`))) ; Fuel Consumption:\n(Fuel Consumption Amount) x (Fuel Consumption Rate)
                (`KismetSystemLibrary.Delay` (`self.Fuel Consumption Rate`))
                ;[1 0 0] Debug fuel.
                (if (`self.Debug: Print Out Fuel Levels`)
                  (if (<= _current_fuel 0.0)
                    (`KismetSystemLibrary.PrintString` "No fuel. Have a nice day." true true (struct :`R` 1.0 :`A` 1.0) 3.0)
                    (goto _label_2)
                    (else
                      (`KismetSystemLibrary.PrintString` (`KismetStringLibrary.Concat_StrStr` "Jetpack fuel:" (`KismetStringLibrary.Conv_DoubleToString` _current_fuel)) true true (struct :`R` 1.0 :`A` 1.0) 1.0)
                      (goto _label_2)))
                  (else
                    (goto _label_2)))
                (else
                  _)))
            (set `self.Consuming Fuel` false :!label _label_3) ; At this point, the player has released their\ninput, or- has run out of fuel from a fuel\nconsuption cycle This begins the shut-down\nsequence.
            (`self.Jetpack Thrust End`) ; This function is what gets carried out when the player stops boosting.\nThis makes sure that the player is not flying towards infinity with one boost.
            (else
              ;[1 0 0] Activate / Deactivate Jetpack (no fuel).
              (`self.Jetpack Thrust Begin` :!label _label_4) ; This function carries out the actual boost.
              (if (`self.Applying Force`)
                (`KismetSystemLibrary.Delay` (`self.No Fuel Force Delay`))
                (goto _label_4))))))
      (:`NewEnumerator3`
        ;[1 0 0] Double Jump Method
        (`KismetSystemLibrary.Delay` 0.01) ; This area is dedicated to secondary function of the Jetpack Blueprint System: the Double Jump.\nThe system supports a practically unlimited number of successive short-lived boosts in the air.\nT he system keeps track of the number of jumps the player has made while in the air, and prevents them\nfrom making additional ones. There is also controls for how the jump behaves, with optional variables for\nlimiting the player's air control, and changing the gravity shortly after they engage another jump.\n\nExtremely slight delay to compensate for the fact the player is still qualified as on the ground while jumping.
        (set `self.Jump Count` (+ (`self.Jump Count`) 1.0)) ; +1 to the number of jumps the player has.
        (`KismetSystemLibrary.Delay` (`self.Jump Delay`)) ; Check if player is still trying to "double jump", use jetpack, after delay.
        (if (and (> (`self.Jump Count`) 1.0) (< (`self.Jump Count`) (`KismetMathLibrary.Conv_IntToDouble` (+ (`self.Max Number of Jumps`) 1))))
          (if (`self.Double Jump Over`)
            (set `CharacterMovementComponent.AirControl` (`self.Flight Air Control`) (`self.Character Movement`)) ; Reset air control.
            (set `CharacterMovementComponent.GravityScale` (`self.Base Gravity`) (`self.Character Movement`)) ; Reset gravity.
          )
          (`Character.LaunchCharacter` (cast `Character` (`self.GetOwner`) :!pure true) (`KismetMathLibrary.MakeVector` 0.0 0.0 (`self.Double Jump Strength`)) false true) ; This is the actual additional jump. Z override is on so that high fall gravity after the first jump don't cancel out subsequent ones.
          (set `CharacterMovementComponent.AirControl` (`self.Flight Air Control`) (`self.Character Movement`)) ; Set the air control the player has while using the jetpack.
          ;[1 0 0] Double jump end delay.
          (`KismetSystemLibrary.RetriggerableDelay` (`self.Double Jump End Delay`))
          (set `self.Double Jump Over` true)
          (if (not (== (`self.Fall Gravity`) 0.0))
            (set `CharacterMovementComponent.GravityScale` (`self.Fall Gravity`) (`self.Character Movement`)))
          (if (`self.Air Control Reset`)
            (set `CharacterMovementComponent.AirControl` (`self.Base Air Control`) (`self.Character Movement`))))))))

(event `/Game/JetpackBPSystem/Blueprints/BPI_Jetpack_ComponentCommunication.BPI Released Jump`
  ;[1 0 0] Check if Jetpack is equipped.
  (if (`self.Jetpack Equipped`)
    ;[1 0 0] Check input method, from there, determine the course of action.
    (switch `/Game/JetpackBPSystem/Blueprints/Enum_JetpackInputMethod` (`self.Input Method`) ; Split the event processing based on what the Input Method is.
      (:`NewEnumerator0`
        ;[1 0 0] Timed lock so "Fall Gravity" doesn't kick in immediately after trying to jump.
        (if (> (`self.Jump Count`) 1.0)
          ;[1 0 0] Do we use fuel?
          (if (> (`self.Max Fuel`) 0.0)
            (goto _label_3)
            (else
              _)))
        ;[1 0 0] Activate / Deactivate Jetpack (no fuel).
        (`self.Jetpack Thrust End` :!label _label_5) ; This function is what gets carried out when the player stops boosting.\nThis makes sure that the player is not flying towards infinity with one boost.
      ))))

(event `/Game/JetpackBPSystem/Blueprints/BPI_Jetpack_ComponentCommunication.BPI Pressed Jetpack`
  ;[1 0 0] Check if Jetpack is equipped.
  (if (`self.Jetpack Equipped`)
    ;[1 0 0] "'Jetpack' input action mapping." input method.
    (switch `/Game/JetpackBPSystem/Blueprints/Enum_JetpackInputMethod` (`self.Input Method`) ; Split the event processing based on what the Input Method is.
      (:`NewEnumerator1`
        ;[1 0 0] Do we use fuel?
        (if (> (`self.Max Fuel`) 0.0)
          (goto _label)
          (else
            (goto _label_4)))))))

(event `/Game/JetpackBPSystem/Blueprints/BPI_Jetpack_ComponentCommunication.BPI Released Jetpack`
  ;[1 0 0] Check if Jetpack is equipped.
  (if (`self.Jetpack Equipped`)
    ;[1 0 0] "'Jetpack' input action mapping." input method.
    (switch `/Game/JetpackBPSystem/Blueprints/Enum_JetpackInputMethod` (`self.Input Method`) ; Split the event processing based on what the Input Method is.
      (:`NewEnumerator1`
        ;[1 0 0] Do we use fuel?
        (if (> (`self.Max Fuel`) 0.0)
          (goto _label_3)
          (else
            (goto _label_5)))))))

(event `CEv: Refuel Check`
  ;[1 0 0] Refuel when on the ground.
  (if (> (`self.Max Fuel`) 0.0)
    (if (`NavMovementComponent.IsFalling` (`self.Character Movement`)) :!label _label_6
      (set `self.Refueling` false) ; Falling / jumping.
      (`KismetSystemLibrary.Delay` (`self.Ground Refuel Rate`)) ; Wait till the player IS on the ground.
      (goto _label_6)
      (else
        (set `self.Refueling` true) ; On the ground.
        (set `self.Current Fuel` (+ (`self.Current Fuel`) (`self.Ground Refuel Amount`))) ; Refuel on ground.
        (if (> (`self.Current Fuel`) (`self.Max Fuel`))
          (set `self.Current Fuel` (`self.Max Fuel`)) ; Current fuel cannot exceed max fuel.
        )
        (`KismetSystemLibrary.Delay` (`self.Ground Refuel Rate`)) ; This delay is for how long until the\nnext cycle of refueling. The shorter\nit is, the faster the player will refuel.
        ;[1 0 0] Debug fuel.
        (if (`self.Debug: Print Out Fuel Levels`)
          (`KismetSystemLibrary.PrintString` (`KismetStringLibrary.Concat_StrStr` "Jetpack fuel:" (`KismetStringLibrary.Conv_DoubleToString` (`self.Current Fuel`))) true true (struct :`R` 1.0 :`G` 0.180137 :`A` 1.0) 1.0)
          (goto _label_6)
          (else
            (goto _label_6)))))))

(fn `Jetpack Check Landed`
  (if (== (`NavMovementComponent.IsFalling` (`self.Character Movement`)) false)
    (`/Engine/EditorBlueprintResources/StandardMacros.DoOnce` false :!label _label ; Don't call too much.
      (:`Completed`
        (`self.Jetpack Landed`)
        (return)))
    (else
      (goto _label :!via `Reset`))))

(fn `Jetpack Landed`
  (if (`self.Jetpack Equipped`)
    (set `self.Consuming Fuel` false) ; Turn off jetpack.
    (set `self.Double Jump Over` false) ; Turn off Double Jump
    (set `self.Jump Count` 0.0) ; Reset the jump count.
    (if (not (== (`self.Fall Gravity`) 0.0))
      (set `CharacterMovementComponent.GravityScale` (`self.Base Gravity`) (`self.Character Movement`)) ; ... take a moment to reset\ngravity to it's base value.
    )
    (set `CharacterMovementComponent.AirControl` (`self.Base Air Control`) (`self.Character Movement`)) ; Equally, reset the air control.
  ))

(fn `Jetpack Thrust Begin`
  (bind _returnvalue (`self.GetOwner`))
  (bind _returnvalue_2 (`Actor.K2_GetActorLocation` _returnvalue))
  (bind _returnvalue_3 (`KismetMathLibrary.GreaterGreater_VectorRotator` (`self.Force Applied`) (`KismetMathLibrary.Conv_VectorToRotator` (`Actor.GetActorForwardVector` _returnvalue))))
  (switch `/Game/JetpackBPSystem/Blueprints/Enum_JetpackFlightMethod` (`self.Flight Method`)
    (:`NewEnumerator0`
      (set `self.Applying Force` true)
      (`CharacterMovementComponent.AddImpulse` (`self.Character Movement`) _returnvalue_3 true)
      (if (`self.Debug: Show Applied Force`)
        (`KismetSystemLibrary.DrawDebugLine` _returnvalue_2 (+ _returnvalue_2 _returnvalue_3) (struct :`R` 1.0 :`A` 1.0) 1.0 1.0)))
    (:`NewEnumerator1`
      (set `CharacterMovementComponent.GravityScale` (* (`self.Flight Thrust`) -1.0) (`self.Character Movement`)) ; Give jetpack "thrust" through inverse gravity.
    ))
  (set `CharacterMovementComponent.AirControl` (`self.Flight Air Control`) (`self.Character Movement`)) ; Set the air control the player has while using the jetpack.
  (message `/Game/JetpackBPSystem/Blueprints/BPI_Jetpack_ComponentCommunication.BPI Pressed Jetpack` (`self.GetOwner`)))

(fn `Jetpack Thrust End`
  (if (== (`self.Fall Gravity`) 0.0)
    (set `CharacterMovementComponent.GravityScale` (`self.Base Gravity`) (`self.Character Movement`)) ; No: set gravity to normal.
    (elif (> (`self.Jump Count`) 1.0)
      (set `CharacterMovementComponent.GravityScale` (`self.Fall Gravity`) (`self.Character Movement`)) ; Yes: set gravity to "Fall Gravity".
    ))
  (set `CharacterMovementComponent.AirControl` (`self.Base Air Control`) (`self.Character Movement`)) ; Set fall control to normal.
  (set `self.Applying Force` false)
  (message `/Game/JetpackBPSystem/Blueprints/BPI_Jetpack_ComponentCommunication.BPI Released Jetpack` (`self.GetOwner`)))