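; BP_MasterAmmoPickup is the base ammo pickup that handles the proximity prompt for picking up ammo.
; When a BP_VystudioCharacterController enters the sphere, it stores that reference, shows the widget, turns on the mesh's custom depth, enables player input and adds a BP_PressActionUI to the viewport.
; Leaving hides the widget, clears custom depth and removes the prompt, but input stays enabled.
; The pickup action itself is not implemented here.
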(event `self.Sphere.OnComponentBeginOverlap`
  (params (OverlappedComponent :type "PrimitiveComponent Object Reference") (OtherActor :type "Actor Object Reference") (OtherComp :type "PrimitiveComponent Object Reference") (OtherBodyIndex :type Integer) (bFromSweep :type Boolean) (SweepResult :type "HitResult Structure (by ref)"))
  (bind _returnvalue (`GameplayStatics.GetPlayerController` 0))
  ;[1 1 1] Visibility Widget and can Pick Up
  (bind _asbp_vystudio_character_controller (cast `/Game/GameCharacterController/Controllers/CharBlueprints/BP_VystudioCharacterController` OtherActor))
  (set `self.VSRef` _asbp_vystudio_character_controller)
  (`SceneComponent.SetVisibility` (`self.Widget`) true false)
  (`PrimitiveComponent.SetRenderCustomDepth` (`self.StaticMesh`) true)
  (`self.EnableInput` _returnvalue)
  (bind _returnvalue_2 (`|CreateWidget` "/Game/GameCharacterController/Controllers/Interface/Help/BP_PressActionUI.BP_PressActionUI_C" _returnvalue))
  (bind _output_get (set `self.ActionWidget` _returnvalue_2))
  (`UserWidget.AddToViewport` _output_get 0))

(event `self.Sphere.OnComponentEndOverlap`
  (params (OverlappedComponent :type "PrimitiveComponent Object Reference") (OtherActor :type "Actor Object Reference") (OtherComp :type "PrimitiveComponent Object Reference") (OtherBodyIndex :type Integer))
  ;[1 1 1] Visibility Widget and can Pick Up
  (bind _asbp_vystudio_character_controller (cast `/Game/GameCharacterController/Controllers/CharBlueprints/BP_VystudioCharacterController` OtherActor))
  (set `self.VSRef` _asbp_vystudio_character_controller)
  (`SceneComponent.SetVisibility` (`self.Widget`) false false)
  (`PrimitiveComponent.SetRenderCustomDepth` (`self.StaticMesh`) false)
  (`Widget.RemoveFromParent` (`self.ActionWidget`)))

(event `InputAction|ItemInteraction`
  (params (Key :type "Key Structure"))
  ;[1 1 1] Visibility Widget and can Pick Up
)

(fn `UserConstructionScript`)