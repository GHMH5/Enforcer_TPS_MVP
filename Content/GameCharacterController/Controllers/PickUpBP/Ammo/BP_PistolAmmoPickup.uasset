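; Pistol ammo pickup that refills the reserve ammo of the pistol held in VSRef when the ItemInteraction input is pressed.
; PickupAmmo doubles as amount and cap: a matching MaxAmmo prints "Full ammo", otherwise the sum is capped at PickupAmmo, effectively setting MaxAmmo to that value for non-negative ammo.
; A successful pickup plays a sound, destroys the actor and hides the action widget.
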(event `InputAction|ItemInteraction`
  (params (Key :type "Key Structure"))
  (bind _iteminfo (`/Game/GameCharacterController/Controllers/WeaponBP/Weapons/BP_Weapon.ItemInfo` (`/Game/GameCharacterController/Controllers/CharBlueprints/BP_VystudioCharacterController.PistolBP` (`self.VSRef`))))
  (bind ((`MaxAmmo_10_ECA372EF47C27FFD0819B6AF15E27DFD` _maxammo)) (break `/Game/GameCharacterController/Controllers/WeaponBP/Other/ItemTypeWeapon` (`/Game/GameCharacterController/Controllers/WeaponBP/Weapons/BP_Weapon.ItemInfo` (`/Game/GameCharacterController/Controllers/CharBlueprints/BP_VystudioCharacterController.PistolBP` (`self.VSRef`)))))
  (bind _returnvalue (+ (`self.PickupAmmo`) _maxammo))
  ;[1 1 1] Calculate Max ammo (pistol ammo + pickup ammo)
  (:`Pressed`
    (if (`KismetSystemLibrary.IsValid` (`/Game/GameCharacterController/Controllers/CharBlueprints/BP_VystudioCharacterController.PistolBP` (`self.VSRef`)))
      (if (== _maxammo (`self.PickupAmmo`))
        (`KismetSystemLibrary.PrintString` "Full ammo")
        (else
          (if (>= _returnvalue (`self.PickupAmmo`))
            (setmembers `/Game/GameCharacterController/Controllers/WeaponBP/Other/ItemTypeWeapon` :`StructRef` _iteminfo :`MaxAmmo` (`self.PickupAmmo`))
            (else
              (setmembers `/Game/GameCharacterController/Controllers/WeaponBP/Other/ItemTypeWeapon` :`StructRef` _iteminfo :`MaxAmmo` _returnvalue)))
          (`GameplayStatics.PlaySound2D` null)
          (`self.K2_DestroyActor`)
          (`Widget.SetVisibility` (`self.ActionWidget`) "Hidden"))))))

(fn `UserConstructionScript`
  (`parent.UserConstructionScript`))