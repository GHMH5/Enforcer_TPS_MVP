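; Pickup-and-fire weapon actor for the Vystudio character controller, covering pistols and rifles.
; An overlap sphere shows an outline and prompt, letting players pick it up.
; Gates drive single or automatic fire, spawning bullets from the muzzle toward a camera trace, with growing rifle spread.
; Empty clips auto-reload using montages, timed magazine drop and swap visuals, and either realistic (discarding leftover rounds) or standard ammo math.
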(event `self.Sphere.OnComponentBeginOverlap`
  (params (OverlappedComponent :type "PrimitiveComponent Object Reference") (OtherActor :type "Actor Object Reference") (OtherComp :type "PrimitiveComponent Object Reference") (OtherBodyIndex :type Integer) (bFromSweep :type Boolean) (SweepResult :type "HitResult Structure (by ref)"))
  (bind _returnvalue (`GameplayStatics.GetPlayerController` 0))
  ;[1 1 1] Pick Up
  (bind _asbp_vystudio_character_controller (cast `/Game/GameCharacterController/Controllers/CharBlueprints/BP_VystudioCharacterController` OtherActor))
  (set `self.VSRef` _asbp_vystudio_character_controller)
  (`SceneComponent.SetVisibility` (`self.Widget`) true false)
  (`self.On/OffVisibilityCustomDepth` true true)
  (`PrimitiveComponent.SetRenderCustomDepth` (`self.SkeletalMesh`) true)
  (set `self.CanWePick?` true)
  (`self.EnableInput` _returnvalue)
  (bind _returnvalue_2 (`|CreateWidget` "/Game/GameCharacterController/Controllers/Interface/Help/BP_PressActionUI.BP_PressActionUI_C" _returnvalue))
  (bind _output_get (set `self.ActionWidget` _returnvalue_2))
  (`UserWidget.AddToViewport` _output_get 0))

(event `self.Sphere.OnComponentEndOverlap`
  (params (OverlappedComponent :type "PrimitiveComponent Object Reference") (OtherActor :type "Actor Object Reference") (OtherComp :type "PrimitiveComponent Object Reference") (OtherBodyIndex :type Integer))
  ;[1 1 1] Pick Up
  (bind _asbp_vystudio_character_controller (cast `/Game/GameCharacterController/Controllers/CharBlueprints/BP_VystudioCharacterController` OtherActor))
  (set `self.VSRef` _asbp_vystudio_character_controller)
  (`SceneComponent.SetVisibility` (`self.Widget`) false false)
  (`self.On/OffVisibilityCustomDepth` false)
  (set `self.CanWePick?` false)
  (`Widget.RemoveFromParent` (`self.ActionWidget`)))

(event `InputAction|ItemInteraction`
  (params (Key :type "Key Structure"))
  ;[1 1 1] Weapon interaction
  (:`Pressed`
    (if (`self.CanWePick?`)
      (`/Game/GameCharacterController/Controllers/CharBlueprints/BP_VystudioCharacterController.PickupWeapon` (`self.VSRef`) self))))

(event `DestroySphere`
  ;[1 1 1] Weapon interaction
  (`ActorComponent.K2_DestroyComponent` (`self.Sphere`)))

(event `PlayAnimIdle`
  ;[1 1 1] Weapon idle Animation
  (`self.AnimIdle`))

(event `AllOff`
  ;[1 1 1] Weapon interaction
  (`self.On/OffVisibilityCustomDepth` false)
  (`SceneComponent.SetVisibility` (`self.Sphere`) false false)
  (`SceneComponent.SetVisibility` (`self.Widget`) false false)
  (`Widget.RemoveFromParent` (`self.ActionWidget`)))

(event `StopFire`
  (bind _vsref (`self.VSRef`))
  (bind _vsref_2 (`self.VSRef`))
  (bind _skeletalmesh (`self.SkeletalMesh`))
  (bind _vsref_3 (`self.VSRef`))
  ;[1 1 1] Fire
  (`|ExecutionSequence`
    (:`then_0`
      ;;[1 1 1] Pistol
      (set `/Game/GameCharacterController/Controllers/CharBlueprints/BP_VystudioCharacterController.shoot` false (`self.VSRef`))
      (goto _label :!via `Close`))
    (:`then_1`
      ;;[1 1 1] Rifle
      (set `/Game/GameCharacterController/Controllers/CharBlueprints/BP_VystudioCharacterController.shoot` false (`self.VSRef`))
      (goto _label_3 :!via `Close`))))

(event `StartFire`
  (bind _vsref (`self.VSRef`))
  (bind _vsref_2 (`self.VSRef`))
  (bind _skeletalmesh (`self.SkeletalMesh`))
  (bind _vsref_3 (`self.VSRef`))
  ;[1 1 1] Fire
  (switch `/Game/GameCharacterController/Controllers/WeaponBP/Other/WeaponType` (`/Game/GameCharacterController/Controllers/CharBlueprints/BP_VystudioCharacterController.WeaponType` (`self.VSRef`))
    (:`NewEnumerator1`
      ;;[1 1 1] Pistol
      (set `self.BulletDegrees` 0.0)
      (`|ExecutionSequence`
        (:`then_0`
          (goto _label :!via `Open`))
        (:`then_1`
          (`/Engine/EditorBlueprintResources/StandardMacros.Gate` true :!label _label
            (:`Exit`
              (`|ExecutionSequence`
                (:`then_1`
                  (if (or (`/Game/GameCharacterController/Controllers/CharBlueprints/BP_VystudioCharacterController.IsDeath?` _vsref_3) (not (`/Game/GameCharacterController/Controllers/CharBlueprints/BP_VystudioCharacterController.IsAim` _vsref_3)))
                    _
                    (elif (<= (`.CurrentAmmo_8_5EF143004EA57AFA774E2186D87FA8DB` (break `/Game/GameCharacterController/Controllers/WeaponBP/Other/ItemTypeWeapon` (`self.ItemInfo`))) 0)
                      (set `self.NotAmmo` true)
                      (set `/Game/GameCharacterController/Controllers/CharBlueprints/BP_VystudioCharacterController.shoot` false (`self.VSRef`))
                      (set `self.CanFire` false)
                      (`KismetSystemLibrary.PrintString` "OUT OF AMMOS" true true (struct :`R` 1.0 :`B` 0.092353 :`A` 1.0))
                      (`self.AnimWithoutAmmo`)
                      (`GameplayStatics.PlaySound2D` (`self.EmptyAmmoSound`))
                      (else
                        ;;[1 1 1] Shoot logic
                        (bind _returnvalue (`self.BulletTrace` :!label _label_2))
                        (`|SpawnActorFromClass` (`self.BulletClass`) _returnvalue "AdjustIfPossibleButDontSpawnIfColliding" "OverrideRootScale" null null)
                        (setmembers `/Game/GameCharacterController/Controllers/WeaponBP/Other/ItemTypeWeapon` :`StructRef` (`self.ItemInfo`) :`CurrentAmmo` (- (`.CurrentAmmo_8_5EF143004EA57AFA774E2186D87FA8DB` (break `/Game/GameCharacterController/Controllers/WeaponBP/Other/ItemTypeWeapon` (`self.ItemInfo`))) 1))
                        (`GameplayStatics.PlaySound2D` (`self.FireSound`))
                        (`Character.PlayAnimMontage` (`self.VSRef`) (`self.PlayFireAnim`) 1.0 "None")
                        (`GameplayStatics.SpawnEmitterAttached` (`self.ShootEffect`) (`self.SkeletalMesh`) (`self.MuzzleSocket`) (`SceneComponent.GetSocketLocation` _skeletalmesh (`self.MuzzleSocket`)) (`SceneComponent.GetSocketRotation` _skeletalmesh (`self.MuzzleSocket`)) (1.0 1.0 1.0) "KeepWorldPosition")
                        (`self.AnimFire`)
                        (set `/Game/GameCharacterController/Controllers/CharBlueprints/BP_VystudioCharacterController.shoot` true (`self.VSRef`))
                        (`Pawn.AddControllerPitchInput` _vsref_2 (+ (`/Game/GameCharacterController/Controllers/CharBlueprints/BP_VystudioCharacterController.AxisValueLookUp` _vsref_2) -0.2))
                        (`KismetSystemLibrary.Delay` 0.01)
                        (set `/Game/GameCharacterController/Controllers/CharBlueprints/BP_VystudioCharacterController.shoot` false (`self.VSRef`))))))))))))
    (:`NewEnumerator2`
      ;;[1 1 1] Rifle
      (set `self.BulletDegrees` 0.0)
      (`|ExecutionSequence`
        (:`then_0`
          (goto _label_3 :!via `Open`))
        (:`then_1`
          (`/Engine/EditorBlueprintResources/StandardMacros.Gate` true :!label _label_3
            (:`Exit`
              (`|ExecutionSequence`
                (:`then_0`
                  (if (`/Game/GameCharacterController/Controllers/CharBlueprints/BP_VystudioCharacterController.AutoFire` (`self.VSRef`))
                    (`KismetSystemLibrary.Delay` 0.2)
                    (`self.ScatterofBullet`
                      (:`Out`
                        (goto _label_3)))))
                (:`then_1`
                  (if (or (`/Game/GameCharacterController/Controllers/CharBlueprints/BP_VystudioCharacterController.IsDeath?` _vsref) (not (`/Game/GameCharacterController/Controllers/CharBlueprints/BP_VystudioCharacterController.IsAim` _vsref)))
                    _
                    (elif (<= (`.CurrentAmmo_8_5EF143004EA57AFA774E2186D87FA8DB` (break `/Game/GameCharacterController/Controllers/WeaponBP/Other/ItemTypeWeapon` (`self.ItemInfo`))) 0)
                      (`KismetSystemLibrary.PrintString` "OUT OF AMMOS" true true (struct :`R` 1.0 :`B` 0.092353 :`A` 1.0))
                      (set `self.NotAmmo` true)
                      (`self.AnimWithoutAmmo`)
                      (set `/Game/GameCharacterController/Controllers/CharBlueprints/BP_VystudioCharacterController.shoot` false (`self.VSRef`))
                      (if (`self.CanFire`)
                        (set `self.AutoFire` true)
                        (else
                          (set `self.AutoFire` false)
                          (`GameplayStatics.PlaySound2D` (`self.EmptyAmmoSound`) 0.3 0.0)))
                      (else
                        (goto _label_2)))))))))))))

(event `FirePress`
  ;[1 1 1] Press or release Fire
  (set `self.CanFire` true)
  (if (not (`self.IsReloading`))
    (if (`/Game/GameCharacterController/Controllers/CharBlueprints/BP_VystudioCharacterController.Pistol` (`self.VSRef`))
      _
      (else
        _))
    (`self.StartFire`)))

(event `FireRelease`
  ;[1 1 1] Press or release Fire
  (set `self.CanFire` false)
  (if (`/Game/GameCharacterController/Controllers/CharBlueprints/BP_VystudioCharacterController.Pistol` (`self.VSRef`))
    _
    (else
      _))
  (`self.StopFire`)
  (`self.AutoReload`))

(event `AutoReload`
  ;[1 1 1] Autoreload. When current ammo = 0
  (if (== (`.CurrentAmmo_8_5EF143004EA57AFA774E2186D87FA8DB` (break `/Game/GameCharacterController/Controllers/WeaponBP/Other/ItemTypeWeapon` (`self.ItemInfo`))) 0)
    (if (== (`.MaxAmmo_10_ECA372EF47C27FFD0819B6AF15E27DFD` (break `/Game/GameCharacterController/Controllers/WeaponBP/Other/ItemTypeWeapon` (`self.ItemInfo`))) 0)
      (`KismetSystemLibrary.PrintString` "Find Ammo")
      (else
        (set `self.IsReloading` true)
        (set `/Game/GameCharacterController/Controllers/CharBlueprints/BP_VystudioCharacterController.IsReloading?` true (`self.VSRef`))
        (`self.Reloading`)
        (`KismetSystemLibrary.Delay` 2.8) ; Reloading Animation Time
        (set `self.IsReloading` false)
        (set `/Game/GameCharacterController/Controllers/CharBlueprints/BP_VystudioCharacterController.IsReloading?` false (`self.VSRef`))))))

(event `Reloading`
  (bind ((`ClipSize_25_350D8D5E4A8B8101D6539094867244EE` _clipsize) (`CurrentAmmo_8_5EF143004EA57AFA774E2186D87FA8DB` _currentammo)) (break `/Game/GameCharacterController/Controllers/WeaponBP/Other/ItemTypeWeapon` (`self.ItemInfo`)))
  ;[1 1 1] Reloading process
  (if (== (`.MaxAmmo_10_ECA372EF47C27FFD0819B6AF15E27DFD` (break `/Game/GameCharacterController/Controllers/WeaponBP/Other/ItemTypeWeapon` (`self.ItemInfo`))) 0)
    (`KismetSystemLibrary.PrintString` "Find Ammo")
    (set `self.NotAmmo` true)
    (else
      (set `self.NotAmmo` false)
      (if (== _clipsize _currentammo)
        (`KismetSystemLibrary.PrintString` "Full Ammo")
        (else
          (bind _output_get (set `self.IsReloading` true))
          (set `/Game/GameCharacterController/Controllers/CharBlueprints/BP_VystudioCharacterController.IsReloading?` true (`self.VSRef`))
          (if _output_get
            (`self.WeaponReload`)
            (`self.AnimReloadPistol`)
            (`self.WeaponReloading`)
            (set `self.IsReloading` false)
            (set `/Game/GameCharacterController/Controllers/CharBlueprints/BP_VystudioCharacterController.IsReloading?` false (`self.VSRef`))
            (`self.AnimIdle`)))))))

(event `WeaponReload`
  (bind _iteminfo (`self.ItemInfo`))
  (bind _vsref (`self.VSRef`))
  (bind _neededammo (`self.NeededAmmo`))
  (bind _iteminfo_2 (`self.ItemInfo`))
  (bind _vsref_2 (`self.VSRef`))
  (bind ((`ClipSize_25_350D8D5E4A8B8101D6539094867244EE` _clipsize) (`CurrentAmmo_8_5EF143004EA57AFA774E2186D87FA8DB` _currentammo)) (break `/Game/GameCharacterController/Controllers/WeaponBP/Other/ItemTypeWeapon` (`self.ItemInfo`)))
  (bind ((`MaxAmmo_10_ECA372EF47C27FFD0819B6AF15E27DFD` _maxammo)) (break `/Game/GameCharacterController/Controllers/WeaponBP/Other/ItemTypeWeapon` (`self.ItemInfo`)))
  (bind ((`ClipSize_25_350D8D5E4A8B8101D6539094867244EE` _clipsize_2) (`MaxAmmo_10_ECA372EF47C27FFD0819B6AF15E27DFD` _maxammo_2)) (break `/Game/GameCharacterController/Controllers/WeaponBP/Other/ItemTypeWeapon` (`self.ItemInfo`)))
  (bind ((`ClipSize_25_350D8D5E4A8B8101D6539094867244EE` _clipsize_3) (`CurrentAmmo_8_5EF143004EA57AFA774E2186D87FA8DB` _currentammo_2)) (break `/Game/GameCharacterController/Controllers/WeaponBP/Other/ItemTypeWeapon` (`self.ItemInfo`)))
  (bind ((`CurrentAmmo_8_5EF143004EA57AFA774E2186D87FA8DB` _currentammo_3) (`MaxAmmo_10_ECA372EF47C27FFD0819B6AF15E27DFD` _maxammo_3)) (break `/Game/GameCharacterController/Controllers/WeaponBP/Other/ItemTypeWeapon` (`self.ItemInfo`)))
  (bind _isaim (`/Game/GameCharacterController/Controllers/CharBlueprints/BP_VystudioCharacterController.IsAim` (`self.VSRef`)))
  ;[1 1 1] Weapon reload (Anim montage, calculate results)
  (if (not (`self.CanFire`))
    (if (`/Game/GameCharacterController/Controllers/CharBlueprints/BP_VystudioCharacterController.Rifle` (`self.VSRef`))
      (if _isaim
        _
        (else
          _))
      (`Character.PlayAnimMontage` _vsref (`/Game/GameCharacterController/Controllers/CharBlueprints/BP_VystudioCharacterController.ReloadRifle` _vsref) 0.8 "None")
      (else
        (if _isaim
          _
          (else
            _))
        (`Character.PlayAnimMontage` _vsref_2 (`/Game/GameCharacterController/Controllers/CharBlueprints/BP_VystudioCharacterController.ReloadPistol` _vsref_2) 0.6 "None")))
    (if (`/Game/GameCharacterController/Controllers/CharBlueprints/BP_VystudioCharacterController.RealisticGaming` (`self.VSRef`))
      ;[1 1 1] Calculate ammo (Realistic gaming type)
      (if (> (`.MaxAmmo_10_ECA372EF47C27FFD0819B6AF15E27DFD` (break `/Game/GameCharacterController/Controllers/WeaponBP/Other/ItemTypeWeapon` (`self.ItemInfo`))) 0)
        (set `self.NeededAmmo` (- _clipsize_3 _currentammo_2))
        (if (<= (`.MaxAmmo_10_ECA372EF47C27FFD0819B6AF15E27DFD` (break `/Game/GameCharacterController/Controllers/WeaponBP/Other/ItemTypeWeapon` (`self.ItemInfo`))) (`self.NeededAmmo`))
          (setmembers `/Game/GameCharacterController/Controllers/WeaponBP/Other/ItemTypeWeapon` :`StructRef` _iteminfo :`CurrentAmmo` (`.MaxAmmo_10_ECA372EF47C27FFD0819B6AF15E27DFD` (break `/Game/GameCharacterController/Controllers/WeaponBP/Other/ItemTypeWeapon` (`self.ItemInfo`))))
          (setmembers `/Game/GameCharacterController/Controllers/WeaponBP/Other/ItemTypeWeapon` :`StructRef` _iteminfo :`MaxAmmo` 0)
          (else
            (setmembers `/Game/GameCharacterController/Controllers/WeaponBP/Other/ItemTypeWeapon` :`StructRef` _iteminfo :`MaxAmmo` (- _maxammo_2 _clipsize_2))
            (setmembers `/Game/GameCharacterController/Controllers/WeaponBP/Other/ItemTypeWeapon` :`StructRef` _iteminfo :`CurrentAmmo` _clipsize_2))))
      (elif (> (`.MaxAmmo_10_ECA372EF47C27FFD0819B6AF15E27DFD` (break `/Game/GameCharacterController/Controllers/WeaponBP/Other/ItemTypeWeapon` (`self.ItemInfo`))) 0)
        (set `self.NeededAmmo` (- _clipsize _currentammo))
        (if (<= _maxammo _neededammo)
          (setmembers `/Game/GameCharacterController/Controllers/WeaponBP/Other/ItemTypeWeapon` :`StructRef` _iteminfo_2 :`CurrentAmmo` (+ _currentammo_3 _maxammo_3))
          (setmembers `/Game/GameCharacterController/Controllers/WeaponBP/Other/ItemTypeWeapon` :`StructRef` _iteminfo_2 :`MaxAmmo` 0)
          (else
            (setmembers `/Game/GameCharacterController/Controllers/WeaponBP/Other/ItemTypeWeapon` :`StructRef` _iteminfo_2 :`MaxAmmo` (- _maxammo _neededammo))
            (setmembers `/Game/GameCharacterController/Controllers/WeaponBP/Other/ItemTypeWeapon` :`StructRef` _iteminfo_2 :`CurrentAmmo` (`.ClipSize_25_350D8D5E4A8B8101D6539094867244EE` (break `/Game/GameCharacterController/Controllers/WeaponBP/Other/ItemTypeWeapon` (`self.ItemInfo`))))))))))

(fn `On/OffVisibilityCustomDepth`
  (params (bNewVisibility :type Boolean) (bValue :type Boolean))
  (`SceneComponent.SetVisibility` (`self.Widget`) bNewVisibility false)
  (`PrimitiveComponent.SetRenderCustomDepth` (`self.SkeletalMesh`) bValue))

(fn `UserConstructionScript`
  (bind (_iteminfo_itemtype _iteminfo_itemclass _iteminfo_clipsize _iteminfo_currentammo _iteminfo_maxammo _iteminfo_damage _iteminfo_itemimage _iteminfo_equipsocketname _iteminfo_unequipsocketname) (break `/Game/GameCharacterController/Controllers/WeaponBP/Other/ItemTypeWeapon` (`self.ItemInfo`)))
  (set `self.ItemInfo` (make `/Game/GameCharacterController/Controllers/WeaponBP/Other/ItemTypeWeapon` _iteminfo_itemtype (`GameplayStatics.GetObjectClass` self) _iteminfo_clipsize _iteminfo_currentammo _iteminfo_maxammo _iteminfo_damage _iteminfo_itemimage _iteminfo_equipsocketname _iteminfo_unequipsocketname)))