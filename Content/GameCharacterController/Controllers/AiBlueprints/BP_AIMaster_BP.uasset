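; Master AI enemy character with health, a HUD widget, and a rifle spawned at start that toggles between armed and unarmed sockets.
; Pawn sensing flags a living player as found, while a forward line trace checks for damageable actors and records an enemy location.
; Headshots kill instantly, and other hits reduce health, alert the AI and briefly show the HUD.
; Death ragdolls the mesh, disables capsule collision and displays the victory screen.
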(event `self.ReceiveBeginPlay`
  ;[1 1 1] Begin play
  (set `self.CurrentHealth` (`self.MaxHealth`))
  (bind _asbp_ai_hud (cast `/Game/GameCharacterController/Controllers/AiBlueprints/BP_AI_HUD` (`WidgetComponent.GetUserWidgetObject` (`self.Widget`))))
  (set `/Game/GameCharacterController/Controllers/AiBlueprints/BP_AI_HUD.Owner` self _asbp_ai_hud)
  (`self.SpawnDefaultWeapon`)
  (`SceneComponent.SetVisibility` (`self.Widget`) false false))

(event `/Game/GameCharacterController/Controllers/AiBlueprints/BP_TakeDamage.iTakeDamage`
  (params (BoneName :type Name) (Damage :type "Float (single-precision)"))
  (bind _returnvalue (`GameplayStatics.GetPlayerController` 0))
  (bind _returnvalue_2 (`GameplayStatics.GetPlayerController` 0))
  (bind _currenthealth (`self.CurrentHealth`))
  ;[1 1 1] Damage
  (if (== BoneName "Head")
    (set `self.CurrentHealth` 0.0)
    (else
      (set `self.EnemyFound` true)
      (set `self.CurrentHealth` (- _currenthealth Damage))))
  (if (<= _currenthealth 0.0)
    (set `self.IsDeath?` true)
    (`SkeletalMeshComponent.SetAllBodiesSimulatePhysics` (`self.Mesh`) true)
    (`PrimitiveComponent.SetCollisionEnabled` (`self.CapsuleComponent`) "NoCollision")
    (`SceneComponent.SetVisibility` (`self.Widget`) false false)
    (`WidgetBlueprintLibrary.SetInputMode_UIOnlyEx` _returnvalue)
    (bind _returnvalue_3 (`|CreateWidget` "/Game/Enforcer_MVPTPSDemoCPP/VictoryScreen.VictoryScreen_C" _returnvalue))
    (bind _output_get (set `self.VictoryWidget` _returnvalue_3))
    (`UserWidget.AddToViewport` _output_get 0)
    (`WidgetBlueprintLibrary.SetInputMode_GameOnly` _returnvalue_2)
    (set `PlayerController.bShowMouseCursor` true _returnvalue_2)
    (else
      (set `self.IsDeath?` false)
      (`SceneComponent.SetVisibility` (`self.Widget`) true false)
      (`KismetSystemLibrary.Delay` 2.0)
      (`SceneComponent.SetVisibility` (`self.Widget`) false false))))

(event `SpawnDefaultWeapon`
  ;[1 1 1] Spawn default weapon
  (bind _returnvalue (`|SpawnActorFromClass` (`self.WeaponClass`) (`SceneComponent.K2_GetComponentToWorld` (`self.Sphere`)) "Undefined" "OverrideRootScale" null (struct) null))
  (bind _output_get (set `self.WeaponBP` _returnvalue))
  (`self.K2_AttachToComponent` _output_get (`self.Mesh`) (`self.RifleSocketUnarmed`) "KeepWorld" "KeepWorld" "KeepWorld" true)
  (`PrimitiveComponent.SetSimulatePhysics` (`/Game/GameCharacterController/Controllers/WeaponBP/Weapons/BP_Weapon.SkeletalMesh` _output_get) false)
  (`/Game/GameCharacterController/Controllers/WeaponBP/Weapons/BP_Weapon.DestroySphere` _returnvalue)
  (if (`self.IsDeath?`)
    (`self.K2_AttachToComponent` _returnvalue null (`self.RifleSocketUnarmed`) "KeepWorld" "KeepWorld" "KeepWorld" true)))

(event `Equip/Unequip`
  ;[1 1 1] Equip/Unequip
  (`/Engine/EditorBlueprintResources/StandardMacros.FlipFlop`
    (:`A`
      (`self.K2_AttachToComponent` (`self.WeaponBP`) (`self.Mesh`) (`self.RifleSocketArmed`) "KeepRelative" "KeepRelative" "KeepRelative" true)
      (set `self.EquipWeapon` true))
    (:`B`
      (`self.K2_AttachToComponent` (`self.WeaponBP`) (`self.Mesh`) (`self.RifleSocketUnarmed`) "KeepRelative" "KeepRelative" "KeepRelative" true)
      (set `self.EquipWeapon` false)
      (set `self.EnemyFound` false))))

(event `EnableCombat`
  ;[1 1 1] Combat event
  (`self.PlayAnimMontage` "/Game/GameCharacterController/DemoContent/AnimStarterPack/Equip_Rifle_Standing_Montage_Demo.Equip_Rifle_Standing_Montage_Demo"))

(event `self.PawnSensing.OnSeePawn`
  (params (Pawn :type "Pawn Object Reference"))
  ;[1 1 1] See
  (bind _asbp_vystudio_character_controller (cast `/Game/GameCharacterController/Controllers/CharBlueprints/BP_VystudioCharacterController` Pawn))
  (if (`/Game/GameCharacterController/Controllers/CharBlueprints/BP_VystudioCharacterController.IsDeath?` _asbp_vystudio_character_controller)
    (set `self.EnemyFound` false)
    (else
      (set `self.EnemyFound` true))))

(event `ScanEnemy`
  (bind _visiondirectionarrow (`self.VisionDirectionArrow`))
  (bind _returnvalue (`SceneComponent.K2_GetComponentLocation` _visiondirectionarrow))
  ;[1 1 1] Search player
  (bind (_outhit _returnvalue_2) (`KismetSystemLibrary.LineTraceSingle` _returnvalue (+ _returnvalue (* (`SceneComponent.GetForwardVector` _visiondirectionarrow) 10000.0)) "TraceTypeQuery1" true (`|MakeArray` self :!type "Actor Object Reference")))
  (if _returnvalue_2
    (bind (_bblockinghit _binitialoverlap _time _distance _location _impactpoint _normal _impactnormal _physmat _hitactor) (`GameplayStatics.BreakHitResult` _outhit))
    (if (`KismetSystemLibrary.DoesImplementInterface` _hitactor "/Game/GameCharacterController/Controllers/AiBlueprints/BP_TakeDamage.BP_TakeDamage_C")
      (cast `/Game/GameCharacterController/Controllers/CharBlueprints/BP_VystudioAiController` _hitactor
        (:`then`
          (set `self.EnemayLocation` _impactpoint))
        (:`CastFailed`
          (set `self.EnemayLocation` (0.0 0.0 0.0))))
      (set `self.Active` true)
      (else
        (set `self.Active` false)))))

(fn `UserConstructionScript`)